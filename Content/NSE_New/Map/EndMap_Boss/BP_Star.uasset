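; BP_Star is an actor in the boss end map that runs a timed attack-and-rise sequence with Boss_Broken_Blueprint.
; BeginPlay sets the boss's Attack flag, then after a delay moves the star to a fixed point and enables Up.
; Tick lifts it per frame, clears Attack and sets EndGame after a delay, resetting the star once it passes a height limit.
; A disconnected branch would play BP_LeftHand_Cha's Die UI animation.
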(event `self.ReceiveBeginPlay`
  (`KismetSystemLibrary.Delay` 1.5)
  (bind _returnvalue (`GameplayStatics.GetActorOfClass` "/Game/NSE_New/Map/EndMap_Boss/Boss_Broken_Blueprint.Boss_Broken_Blueprint_C"))
  (set `/Game/NSE_New/Map/EndMap_Boss/Boss_Broken_Blueprint.Attack` true _returnvalue)
  (`KismetSystemLibrary.Delay` 1.5)
  (`self.K2_SetActorLocation` (7379.0 13.0 1526.0))
  (set `self.Up` true))

(event `self.ReceiveTick`
  (params (DeltaSeconds :type "Float (single-precision)"))
  (bind (_returnvalue_x _returnvalue_y _returnvalue_z) (`KismetMathLibrary.BreakVector` (`self.K2_GetActorLocation`)))
  (if (`self.Up`)
    (if (> _returnvalue_z 5000.0)
      (`self.K2_SetActorLocation` (7379.0 13.0 1526.0))
      (set `self.Up` false)
      (else
        (`self.K2_AddActorWorldOffset` (0.0 0.0 30.0))
        (bind _returnvalue (`GameplayStatics.GetActorOfClass` "/Game/NSE_New/Map/EndMap_Boss/Boss_Broken_Blueprint.Boss_Broken_Blueprint_C"))
        (set `/Game/NSE_New/Map/EndMap_Boss/Boss_Broken_Blueprint.Attack` false _returnvalue)
        (`KismetSystemLibrary.Delay` 2.0)
        (set `self.EndGame` true)))))

(fn `UserConstructionScript`)