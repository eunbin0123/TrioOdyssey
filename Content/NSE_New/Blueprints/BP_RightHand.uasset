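; Boss right-hand actor that runs five attack patterns against the player and damages BP_ToBeMario on sphere overlap.
; Tick dispatches on AttackAll to per-attack state machines that move the hand by interpolation and offsets.
; Patterns cover a chasing slam, repeated claps ending in BossMap2 loading, head-following BP_Ice fire, a rising spin-and-sweep, and a straight slam.
; It signals BP_LeftHand_Cha and BP_Head, with StartLoc easing it toward a hard-coded home position.
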(event `Attack1`
  (bind (_returnvalue_x _returnvalue_y _returnvalue_z) (`KismetMathLibrary.BreakVector` (`self.K2_GetActorLocation`)))
  (bind (_returnvalue_roll _returnvalue_pitch _returnvalue_yaw) (`KismetMathLibrary.BreakRotator` (`self.K2_GetActorRotation`)))
  (bind (_returnvalue_x_2 _returnvalue_y_2 _returnvalue_z_2) (`KismetMathLibrary.BreakVector` (`self.K2_GetActorLocation`)))
  (bind (_returnvalue_x_3 _returnvalue_y_3 _returnvalue_z_3) (`KismetMathLibrary.BreakVector` (`self.K2_GetActorLocation`)))
  (bind (_returnvalue_x_4 _returnvalue_y_4 _returnvalue_z_4) (`KismetMathLibrary.BreakVector` (`self.K2_GetActorLocation`)))
  (bind (_returnvalue_roll_2 _returnvalue_pitch_2 _returnvalue_yaw_2) (`KismetMathLibrary.BreakRotator` (`self.K2_GetActorRotation`)))
  (bind (_returnvalue_roll_3 _returnvalue_pitch_3 _returnvalue_yaw_3) (`KismetMathLibrary.BreakRotator` (`self.K2_GetActorRotation`)))
  (bind (_returnvalue_x_5 _returnvalue_y_5) (`KismetMathLibrary.BreakVector` (`self.K2_GetActorLocation` (`GameplayStatics.GetPlayerPawn` 0))))
  (bind (_returnvalue_x_6 _returnvalue_y_6) (`KismetMathLibrary.BreakVector` (`self.K2_GetActorLocation` (`GameplayStatics.GetPlayerPawn` 0))))
  (bind _returnvalue (`KismetMathLibrary.MakeVector` _returnvalue_x_6 _returnvalue_y_6 _returnvalue_z_4))
  (bind (_returnvalue_roll_4 _returnvalue_pitch_4 _returnvalue_yaw_4) (`KismetMathLibrary.BreakRotator` (`KismetMathLibrary.RInterpTo` (`self.K2_GetActorRotation`) (`KismetMathLibrary.FindLookAtRotation` (`self.K2_GetActorLocation` (`GameplayStatics.GetPlayerPawn` 0)) (`self.K2_GetActorLocation`)) (`GameplayStatics.GetWorldDeltaSeconds`) 10.0)))
  (switch `/Game/NSE_New/Animations/ERightAttack1` (`self.State_Attack1`)
    (:`NewEnumerator0`
      (`KismetSystemLibrary.Delay` 2.0)
      (set `self.State_Attack1` "NewEnumerator1"))
    (:`NewEnumerator1`
      (if (< (`KismetMathLibrary.Vector_Distance` (`self.K2_GetActorLocation`) _returnvalue) 300.0)
        ;[1 1 1 0.5] 플레이어와의 거리가 3m 이내이면 멈춘다. 그리고 90도 회전한다.
        (`KismetSystemLibrary.Delay` 1.0)
        (`self.K2_SetActorLocation` (`KismetMathLibrary.MakeVector` _returnvalue_x_5 _returnvalue_y_5 _returnvalue_z))
        (`self.K2_SetActorRotation` (`KismetMathLibrary.RInterpTo` (`self.K2_GetActorRotation`) (`KismetMathLibrary.MakeRotator` _returnvalue_roll 90.0 _returnvalue_yaw) (`GameplayStatics.GetWorldDeltaSeconds`) 100.0))
        (`KismetSystemLibrary.Delay` 0.2)
        (set `self.State_Attack1` "NewEnumerator2")
        (else
          ;[1 1 1 0.5] 플레이어 방향으로 z축 회전
          (`self.K2_SetActorRotation` (`KismetMathLibrary.MakeRotator` 0.0 0.0 _returnvalue_yaw_4))
          ;[1 1 1 0.5] 이동하다가
          (`self.K2_SetActorLocation` (+ (`self.K2_GetActorLocation`) (* (`KismetMathLibrary.Normal` (- _returnvalue (`self.K2_GetActorLocation`))) 400.0 (`GameplayStatics.GetWorldDeltaSeconds`))))
          (`self.K2_SetActorRotation` (`KismetMathLibrary.RInterpTo` (`self.K2_GetActorRotation`) (`KismetMathLibrary.MakeRotator` _returnvalue_roll_2 60.0 _returnvalue_yaw_2) (`GameplayStatics.GetWorldDeltaSeconds`) 40.0)))))
    (:`NewEnumerator2`
      ;[1 1 1] 내려찍기
      (if (< _returnvalue_z_2 10.0)
        (`self.K2_AddActorLocalOffset` (0.0 0.0 0.0))
        (`KismetSystemLibrary.Delay` 1.0)
        (set `self.IsLeftAttack` true)
        (`GameplayStatics.PlaySound2D` "/Game/NSE_New/Sound/FlyingFist.FlyingFist" 1.0 1.0 0.0 null null)
        (set `self.State_Attack1` "NewEnumerator3")
        (else
          (`self.K2_AddActorLocalOffset` (-40.0 0.0 0.0)))))
    (:`NewEnumerator3`
      ;[1 1 1] 제자리로 복귀
      (`self.StartLoc`)
      (if (`self.IsLeftAttack`)
        (bind _outactors (`GameplayStatics.GetAllActorsOfClass` "/Game/NSE_New/Blueprints/BP_LeftHand_Cha.BP_LeftHand_Cha_C"))
        (set `/Game/NSE_New/Blueprints/BP_LeftHand_Cha.IsAttack1` true (`|GetArrayItem` _outactors))))
    (:`NewEnumerator4`
      (bind _output (`|GetArrayItem` (stale _outactors_2)))
      (bind _returnvalue_2 (`self.K2_GetActorLocation` _output))
      (if (< (`KismetMathLibrary.Vector_Distance` (`self.K2_GetActorLocation`) _returnvalue_2) 700.0)
        (`KismetSystemLibrary.Delay` 1.0)
        (`self.K2_SetActorLocation` (`self.K2_GetActorLocation`))
        (set `self.State_Attack1` "NewEnumerator3")
        (else
          ;[1 1 1] Lefthand로 반격
          (bind _outactors_2 (`GameplayStatics.GetAllActorsOfClass` "/Game/NSE_New/Blueprints/BP_LeftHand_Cha.BP_LeftHand_Cha_C"))
          (bind (_returnvalue_roll_5 _returnvalue_pitch_5 _returnvalue_yaw_5) (`KismetMathLibrary.BreakRotator` (`KismetMathLibrary.RInterpTo` (`self.K2_GetActorRotation`) (`KismetMathLibrary.FindLookAtRotation` _returnvalue_2 (`self.K2_GetActorLocation`)) (`GameplayStatics.GetWorldDeltaSeconds`) 10.0)))
          (`self.K2_SetActorRotation` (`KismetMathLibrary.MakeRotator` 0.0 0.0 _returnvalue_yaw_5))
          (bind (_returnvalue_x_7 _returnvalue_y_7) (`KismetMathLibrary.BreakVector` (`self.K2_GetActorLocation` _output)))
          (`self.K2_SetActorLocation` (+ (`self.K2_GetActorLocation`) (* (`KismetMathLibrary.Normal` (- (`KismetMathLibrary.MakeVector` _returnvalue_x_7 _returnvalue_y_7 _returnvalue_z_3) (`self.K2_GetActorLocation`))) 400.0 (`GameplayStatics.GetWorldDeltaSeconds`))))
          (`self.K2_SetActorRotation` (`KismetMathLibrary.RInterpTo` (`self.K2_GetActorRotation`) (`KismetMathLibrary.MakeRotator` _returnvalue_roll_3 60.0 _returnvalue_yaw_3) (`GameplayStatics.GetWorldDeltaSeconds`) 40.0)))))))

(event `Atttack->Locomotion`)

(event `Attack2`
  (bind (_returnvalue_x _returnvalue_y) (`KismetMathLibrary.BreakVector` (`self.K2_GetActorLocation`)))
  (bind _returnvalue_x_2 (`KismetMathLibrary.BreakVector` (`self.K2_GetActorLocation`)))
  (bind (_returnvalue_x_3 _returnvalue_y_2) (`KismetMathLibrary.BreakVector` (`self.K2_GetActorLocation`)))
  (bind (_returnvalue_x_4 _returnvalue_y_3 _returnvalue_z) (`KismetMathLibrary.BreakVector` (`self.K2_GetActorLocation`)))
  (bind (_returnvalue_x_5 _returnvalue_y_4) (`KismetMathLibrary.BreakVector` (`self.K2_GetActorLocation` (`GameplayStatics.GetPlayerPawn` 0))))
  (bind _returnvalue_x_6 (`KismetMathLibrary.BreakVector` (`self.K2_GetActorLocation` (`GameplayStatics.GetPlayerPawn` 0))))
  (bind (_returnvalue_x_7 _returnvalue_y_5) (`KismetMathLibrary.BreakVector` (`self.K2_GetActorLocation` (`GameplayStatics.GetPlayerPawn` 0))))
  (bind (_returnvalue_x_8 _returnvalue_y_6) (`KismetMathLibrary.BreakVector` (`self.K2_GetActorLocation` (`GameplayStatics.GetPlayerPawn` 0))))
  (bind (_returnvalue_x_9 _returnvalue_y_7) (`KismetMathLibrary.BreakVector` (`self.K2_GetActorLocation` (`GameplayStatics.GetPlayerPawn` 0))))
  (bind _returnvalue_x_10 (`KismetMathLibrary.BreakVector` (+ (`self.K2_GetActorLocation`) (* (`KismetMathLibrary.Normal` (- (`KismetMathLibrary.MakeVector` _returnvalue_x_9 _returnvalue_y_7 _returnvalue_z) (`self.K2_GetActorLocation`))) 400.0 (`GameplayStatics.GetWorldDeltaSeconds`)))))
  (switch `/Game/NSE_New/Animations/ERightAttack2` (`self.State_Attack2`)
    (:`NewEnumerator0`
      (set `self.State_Attack2` "NewEnumerator1"))
    (:`NewEnumerator1`
      (if (< (`KismetMathLibrary.Vector_Distance` (`KismetMathLibrary.MakeVector` _returnvalue_x_2) (`KismetMathLibrary.MakeVector` _returnvalue_x_6)) 100.0)
        (`KismetSystemLibrary.Delay` 2.0)
        (set `self.State_Attack2` "NewEnumerator2")
        (else
          ;[1 1 1 0.5] chase
          (`self.K2_SetActorLocation` (`KismetMathLibrary.MakeVector` _returnvalue_x_10 (+ _returnvalue_y_6 -800.0) 170.0))
          (`self.K2_SetActorRotation` (`KismetMathLibrary.RInterpTo` (`self.K2_GetActorRotation`) (`KismetMathLibrary.MakeRotator` 0.0 -90.0 -90.0) (`GameplayStatics.GetWorldDeltaSeconds`) 10.0)))))
    (:`NewEnumerator2`
      ;[1 1 1] 박수치기
      (if (< (`KismetMathLibrary.Vector_Distance` (`KismetMathLibrary.MakeVector` 0.0 _returnvalue_y_2) (`KismetMathLibrary.MakeVector` 0.0 _returnvalue_y_5)) 150.0)
        (`self.K2_AddActorLocalOffset` (0.0 0.0 0.0))
        (`|ExecutionSequence`
          (:`then_0`
            (`ActorComponent.Activate` (`self.ClapFX`) false)
            (`KismetSystemLibrary.Delay` 2.0)
            (set `self.State_Attack2` "NewEnumerator3"))
          (:`then_1`
            (`GameplayStatics.PlaySound2D` "/Game/NSE_New/Sound/Clap.Clap" 1.0 1.0 0.0 null null)))
        (else
          (`self.K2_AddActorLocalOffset` (0.0 0.0 -80.0)))))
    (:`NewEnumerator3`
      ;[1 1 1] 박수쳤다가 떼기
      (`ActorComponent.Deactivate` (`self.ClapFX`))
      (if (< 800.0 (`KismetMathLibrary.Vector_Distance` (`KismetMathLibrary.MakeVector` 0.0 _returnvalue_y) (`KismetMathLibrary.MakeVector` 0.0 _returnvalue_y_4)))
        (`self.K2_AddActorLocalOffset` (0.0 0.0 0.0))
        (set `self.ClapNum` (- (`self.ClapNum`) 1.0))
        (if (< (`self.ClapNum`) 0.0)
          (`GameplayStatics.OpenLevel` "BossMap2")
          (else
            (set `self.State_Attack2` "NewEnumerator1")))
        (else
          (`self.K2_AddActorLocalOffset` (0.0 0.0 40.0)))))))

(event `Attack3`
  (bind _returnvalue_x (`KismetMathLibrary.BreakVector` (`self.K2_GetActorLocation`)))
  (bind (_returnvalue_roll _returnvalue_pitch _returnvalue_yaw) (`KismetMathLibrary.BreakRotator` (`KismetMathLibrary.RInterpTo` (`self.K2_GetActorRotation`) (`KismetMathLibrary.FindLookAtRotation` (`self.K2_GetActorLocation` (`GameplayStatics.GetPlayerPawn` 0)) (`self.K2_GetActorLocation`)) (`GameplayStatics.GetWorldDeltaSeconds`) 5.0)))
  (switch `/Game/NSE_New/Animations/ERightAttack3` (`self.State_Attack3`)
    (:`NewEnumerator0`
      ;[1 1 1 0.5] 제자리로 이동
      (`self.K2_SetActorLocationAndRotation` (+ (`self.K2_GetActorLocation`) (* (`KismetMathLibrary.Normal` (- (`KismetMathLibrary.MakeVector` 6778.0 -998.0 519.0) (`self.K2_GetActorLocation`))) 800.0 (`GameplayStatics.GetWorldDeltaSeconds`))))
      (if (> _returnvalue_x 6770.0)
        (set `self.State_Attack3` "NewEnumerator1")))
    (:`NewEnumerator1`
      ;[1 1 1 0.5] head의 위치를 따라감
      (bind _outactors (`GameplayStatics.GetAllActorsOfClass` "/Game/NSE_New/Blueprints/BP_Head.BP_Head_C"))
      (bind (_returnvalue_x_2 _returnvalue_y) (`KismetMathLibrary.BreakVector` (`self.K2_GetActorLocation` (`|GetArrayItem` _outactors))))
      (`self.K2_SetActorLocation` (`KismetMathLibrary.MakeVector` (+ _returnvalue_x_2 -1200.0) (+ _returnvalue_y -600.0) 519.0))
      ;[1 1 1 0.5] FistAttack3
      (`self.K2_SetActorRotation` (`KismetMathLibrary.MakeRotator` 0.0 0.0 _returnvalue_yaw))
      (`self.MakeIce`))))

(event `self.ReceiveTick`
  (params (DeltaSeconds :type "Float (single-precision)"))
  (switch `/Game/NSE_New/Animations/ERight_All` (`self.Attack_All`)
    (:`NewEnumerator0`
      (`self.Attack1`))
    (:`NewEnumerator1`
      (`self.Attack2`))
    (:`NewEnumerator2`
      (`self.Attack3`))
    (:`NewEnumerator3`
      (`self.Attack4`))
    (:`NewEnumerator4`
      (`self.Attack5`))))

(event `MakeIce`
  (bind (_returnvalue_location _returnvalue_rotation) (`KismetMathLibrary.BreakTransform` (`SceneComponent.K2_GetComponentToWorld` (`self.Arrow`))))
  ;[1 1 1] 얼음 생성
  (`KismetSystemLibrary.Delay` 0.8)
  (`|SpawnActorFromClass` "/Game/NSE_New/Blueprints/BP_Ice.BP_Ice_C" (`KismetMathLibrary.MakeTransform` _returnvalue_location _returnvalue_rotation) "Undefined" "MultiplyWithRoot" null null))

(event `Attack4`
  (bind _returnvalue_x (`KismetMathLibrary.BreakVector` (`self.K2_GetActorLocation`)))
  (bind (_returnvalue_x_2 _returnvalue_y _returnvalue_z) (`KismetMathLibrary.BreakVector` (`self.K2_GetActorLocation`)))
  (switch `/Game/NSE_New/Animations/ERightAttack4` (`self.State_Attack4`)
    (:`NewEnumerator0`
      (bind _outactors (`GameplayStatics.GetAllActorsOfClass` "/Game/NSE_New/Blueprints/BP_Head.BP_Head_C"))
      (bind (_returnvalue_x_3 _returnvalue_y_2 _returnvalue_z_2) (`KismetMathLibrary.BreakVector` (`self.K2_GetActorLocation` (`|GetArrayItem` _outactors))))
      (`self.K2_SetActorLocation` (`KismetMathLibrary.MakeVector` (+ _returnvalue_x_3 -900.0) (+ _returnvalue_y_2 -900.0) (+ _returnvalue_z_2 -2000.0)))
      (set `self.State_Attack4` "NewEnumerator1"))
    (:`NewEnumerator1`
      ;[1 1 1 0.5] 손이 위로 올라오기
      (if (> (+ _returnvalue_z 400.0) _returnvalue_z_2)
        (`self.K2_AddActorWorldOffset` (0.0 0.0 0.0))
        (set `self.State_Attack4` "NewEnumerator2")
        (else
          (`self.K2_AddActorWorldOffset` (0.0 0.0 10.0)))))
    (:`NewEnumerator2`
      (`self.K2_AddActorLocalRotation` (struct :`Roll` -7.0))
      (`KismetSystemLibrary.Delay` 2.0)
      (`self.K2_SetActorRotation` (struct))
      (set `self.State_Attack4` "NewEnumerator3"))
    (:`NewEnumerator3`
      (`ActorComponent.Activate` (`self.NS_WallJump`) false)
      (if (> 13262.0 _returnvalue_x)
        (`self.K2_AddActorWorldOffset` (0.0 0.0 0.0) true)
        (set `self.State_Attack4` "NewEnumerator4")
        (bind _outactors_2 (`GameplayStatics.GetAllActorsOfClass` "/Game/NSE_New/Blueprints/BP_Head.BP_Head_C"))
        (set `/Game/NSE_New/Blueprints/BP_Head.HeadState` "NewEnumerator4" (`|GetArrayItem` _outactors_2))
        (else
          (`self.K2_AddActorWorldOffset` (-50.0 0.0 0.0)))))
    (:`NewEnumerator4`
      (`ActorComponent.Deactivate` (`self.NS_WallJump`))
      (`self.StartLoc`))))

(event `self.ReceiveBeginPlay`
  (`ActorComponent.Deactivate` (`self.NS_WallJump`))
  (`ActorComponent.Deactivate` (`self.ClapFX`)))

(event `Attack5`
  (bind (_returnvalue_x _returnvalue_y _returnvalue_z) (`KismetMathLibrary.BreakVector` (`self.K2_GetActorLocation`)))
  (switch `/Game/NSE_New/Animations/ERightAttack5` (`self.State_Attack5`)
    (:`NewEnumerator0`
      (`self.StartLoc`)
      (`KismetSystemLibrary.Delay` 2.0)
      (set `self.State_Attack5` "NewEnumerator1"))
    (:`NewEnumerator1`
      ;[1 1 1] 내려찍기
      (if (< _returnvalue_z 10.0)
        (`self.K2_AddActorLocalOffset` (0.0 0.0 0.0))
        (`KismetSystemLibrary.Delay` 3.0)
        (set `self.State_Attack5` "NewEnumerator2")
        (else
          (`self.K2_AddActorLocalOffset` (0.0 0.0 -40.0)))))
    (:`NewEnumerator2`
      (`self.StartLoc`))))

(event `self.Sphere.OnComponentBeginOverlap`
  (params (OverlappedComponent :type "PrimitiveComponent Object Reference") (OtherActor :type "Actor Object Reference") (OtherComp :type "PrimitiveComponent Object Reference") (OtherBodyIndex :type Integer) (bFromSweep :type Boolean) (SweepResult :type "HitResult Structure (by ref)"))
  (bind _asbp_to_be_mario (cast `/Game/CJWCharactor/ThirdPerson/Blueprints/BP_ToBeMario` OtherActor))
  (set `/Game/CJWCharactor/ThirdPerson/Blueprints/BP_ToBeMario.IsGetDamage` true _asbp_to_be_mario)
  (set `/Game/CJWCharactor/ThirdPerson/Blueprints/BP_ToBeMario.MaxHp` (- (`/Game/CJWCharactor/ThirdPerson/Blueprints/BP_ToBeMario.MaxHp` _asbp_to_be_mario) 1.0) _asbp_to_be_mario))

(event `self.Sphere.OnComponentEndOverlap`
  (params (OverlappedComponent :type "PrimitiveComponent Object Reference") (OtherActor :type "Actor Object Reference") (OtherComp :type "PrimitiveComponent Object Reference") (OtherBodyIndex :type Integer))
  (bind _asbp_to_be_mario (cast `/Game/CJWCharactor/ThirdPerson/Blueprints/BP_ToBeMario` OtherActor))
  (set `/Game/CJWCharactor/ThirdPerson/Blueprints/BP_ToBeMario.IsGetDamage` false _asbp_to_be_mario))

(fn `StartLoc`
  (`self.K2_SetActorLocationAndRotation` (+ (`self.K2_GetActorLocation`) (* (`KismetMathLibrary.Normal` (- (`KismetMathLibrary.MakeVector` 16040.0 -998.0 519.0) (`self.K2_GetActorLocation`))) 600.0 (`GameplayStatics.GetWorldDeltaSeconds`))))
  (return))

(fn `UserConstructionScript`)