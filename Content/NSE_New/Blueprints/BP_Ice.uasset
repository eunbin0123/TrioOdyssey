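; BP_Ice is an ice actor that flies in a straight line and removes itself shortly after spawning.
; Each tick, Translate offsets its location along the forward vector by Speed scaled by delta time, without sweeping for collision.
; On BeginPlay, a fixed delay runs and then a very short life span is set to destroy the actor.
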(event `self.ReceiveBeginPlay`
  (`KismetSystemLibrary.Delay` 4.0)
  (`self.SetLifeSpan` 0.1))

(event `self.ReceiveTick`
  (params (DeltaSeconds :type "Float (single-precision)"))
  (`self.Translate` (`self.GetActorForwardVector`) (`self.Speed`)))

(fn `Translate`
  (params (Direction :type "Vector Structure") (Speed :type "Float (double-precision)"))
  (`self.K2_SetActorLocation` (+ (`self.K2_GetActorLocation`) (* Direction Speed (`GameplayStatics.GetWorldDeltaSeconds`)))))

(fn `UserConstructionScript`)