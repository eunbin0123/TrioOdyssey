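; BP_SpawnIce is a spawner actor that creates BP_IceFall actors at its Spawn component while the left-hand character's IceFall flag is on.
; Each Tick looks up the first BP_LeftHand_Cha via GetAllActorsOfClass and checks that flag.
; A random roll passes most ticks into a two-second Delay, which throttles calls to the MakeIceSpawn event that performs the spawn.
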(event `Make Ice Spawn`
  (bind (_returnvalue_location _returnvalue_rotation) (`KismetMathLibrary.BreakTransform` (`SceneComponent.K2_GetComponentToWorld` (`self.Spawn`))))
  (`|SpawnActorFromClass` "/Game/NSE_New/Blueprints/BP_IceFall.BP_IceFall_C" (`KismetMathLibrary.MakeTransform` _returnvalue_location _returnvalue_rotation) "Undefined" "MultiplyWithRoot" null null))

(event `self.ReceiveTick`
  (params (DeltaSeconds :type "Float (single-precision)"))
  (`/Engine/EditorBlueprintResources/StandardMacros.IsValid` "/Game/NSE_New/Blueprints/BP_LeftHand_Cha.BP_LeftHand_Cha"
    (:`Is Valid`
      (bind _outactors (`GameplayStatics.GetAllActorsOfClass` "/Game/NSE_New/Blueprints/BP_LeftHand_Cha.BP_LeftHand_Cha_C"))
      (if (`/Game/NSE_New/Blueprints/BP_LeftHand_Cha.IceFall` (`|GetArrayItem` _outactors))
        (if (not (< (`KismetMathLibrary.RandomIntegerInRange` 0 9) 3))
          (`KismetSystemLibrary.Delay` 2.0)
          (`self.Make Ice Spawn`))))))

(fn `UserConstructionScript`)