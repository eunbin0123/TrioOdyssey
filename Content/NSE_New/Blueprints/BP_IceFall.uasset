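; BP_IceFall is a falling ice hazard that damages the BP_ToBeMario player.
; Tick moves it downward at Speed through a Translate helper, without sweep, and resets a short lifespan every frame.
; The particle system starts off and activates when anything overlaps Sphere.
; IceCollision overlap takes one Hp and sets IsGetDamage on that character, clearing the flag when overlap ends.
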(event `self.ReceiveBeginPlay`
  (`ActorComponent.Deactivate` (`self.ParticleSystem`)))

(event `self.ReceiveTick`
  (params (DeltaSeconds :type "Float (single-precision)"))
  (`self.Translate` (0.0 0.0 -10.0) (`self.Speed`))
  (`self.SetLifeSpan` 0.1))

(event `self.Sphere.OnComponentBeginOverlap`
  (params (OverlappedComponent :type "PrimitiveComponent Object Reference") (OtherActor :type "Actor Object Reference") (OtherComp :type "PrimitiveComponent Object Reference") (OtherBodyIndex :type Integer) (bFromSweep :type Boolean) (SweepResult :type "HitResult Structure (by ref)"))
  (`ActorComponent.Activate` (`self.ParticleSystem`) false))

(event `self.IceCollision.OnComponentBeginOverlap`
  (params (OverlappedComponent :type "PrimitiveComponent Object Reference") (OtherActor :type "Actor Object Reference") (OtherComp :type "PrimitiveComponent Object Reference") (OtherBodyIndex :type Integer) (bFromSweep :type Boolean) (SweepResult :type "HitResult Structure (by ref)"))
  (bind _asbp_to_be_mario (cast `/Game/CJWCharactor/ThirdPerson/Blueprints/BP_ToBeMario` OtherActor))
  (set `/Game/CJWCharactor/ThirdPerson/Blueprints/BP_ToBeMario.IsGetDamage` true _asbp_to_be_mario)
  (set `/Game/CJWCharactor/ThirdPerson/Blueprints/BP_ToBeMario.Hp` (- (`/Game/CJWCharactor/ThirdPerson/Blueprints/BP_ToBeMario.Hp` _asbp_to_be_mario) 1.0) _asbp_to_be_mario))

(event `self.IceCollision.OnComponentEndOverlap`
  (params (OverlappedComponent :type "PrimitiveComponent Object Reference") (OtherActor :type "Actor Object Reference") (OtherComp :type "PrimitiveComponent Object Reference") (OtherBodyIndex :type Integer))
  (bind _asbp_to_be_mario (cast `/Game/CJWCharactor/ThirdPerson/Blueprints/BP_ToBeMario` OtherActor))
  (set `/Game/CJWCharactor/ThirdPerson/Blueprints/BP_ToBeMario.IsGetDamage` false _asbp_to_be_mario))

(fn `Translate`
  (params (Direction :type "Vector Structure") (Speed :type "Float (double-precision)"))
  (`self.K2_SetActorLocation` (+ (`self.K2_GetActorLocation`) (* Direction Speed (`GameplayStatics.GetWorldDeltaSeconds`)))))

(fn `UserConstructionScript`)