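; BP_Head is a head actor, apparently part of a boss with left and right hands, driven on Tick by HeadState.
; It yaws along the player-to-head direction, backs away with query collision enabled, flies off spinning when damaged, or moves toward a fixed start point.
; Left-hand overlap triggers near-frozen global time dilation and particles, then a short delay restores time and arms the damaged transition.
; The head also sets the hands' attack states directly.
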(event `self.ReceiveActorBeginOverlap`
  (params (OtherActor :type "Actor Object Reference"))
  (cast `/Game/NSE_New/Blueprints/BP_LeftHand_Cha` OtherActor)
  (if (`self.IsTimeDilated`)
    (`GameplayStatics.SetGlobalTimeDilation` 1.0)
    (set `self.IsTimeDilated` true)
    (else
      (`GameplayStatics.SetGlobalTimeDilation` 0.01)
      (`|ExecutionSequence`
        (:`then_0`
          (bind _outactors (`GameplayStatics.GetAllActorsOfClass` "/Game/NSE_New/Blueprints/BP_LeftHand_Cha.BP_LeftHand_Cha_C"))
          (set `/Game/NSE_New/Blueprints/BP_LeftHand_Cha.State_Attack3` "NewEnumerator1" (`|GetArrayItem` _outactors))
          (`KismetSystemLibrary.Delay` 0.03)
          (set `self.IsTimeDilated` true)
          (`GameplayStatics.SetGlobalTimeDilation` 1.0)
          (set `self.Delayed` true))
        (:`then_1`
          (`ActorComponent.Activate` (`self.ParticleSystem`) false))))))

(event `self.ReceiveBeginPlay`
  (`ActorComponent.Deactivate` (`self.ParticleSystem`)))

(event `self.ReceiveTick`
  (params (DeltaSeconds :type "Float (single-precision)"))
  (bind _returnvalue_x (`KismetMathLibrary.BreakVector` (`self.K2_GetActorLocation`)))
  (bind _returnvalue_x_2 (`KismetMathLibrary.BreakVector` (`self.K2_GetActorLocation`)))
  (bind (_returnvalue_roll _returnvalue_pitch _returnvalue_yaw) (`KismetMathLibrary.BreakRotator` (`KismetMathLibrary.RInterpTo` (`self.K2_GetActorRotation`) (`KismetMathLibrary.FindLookAtRotation` (`self.K2_GetActorLocation` (`GameplayStatics.GetPlayerPawn` 0)) (`self.K2_GetActorLocation`)) (`GameplayStatics.GetWorldDeltaSeconds`) 10.0)))
  (switch `/Game/NSE_New/Animations/EHeadAttack_All` (`self.HeadState`)
    (:`NewEnumerator0`
      (`PrimitiveComponent.SetCollisionEnabled` (`self.Sphere`) "NoCollision")
      ;[1 1 1 0.5] 기본 도리도리
      (`self.K2_SetActorRotation` (`KismetMathLibrary.MakeRotator` 0.0 0.0 _returnvalue_yaw))
      (`KismetSystemLibrary.Delay` 2.0))
    (:`NewEnumerator1`
      (`PrimitiveComponent.SetCollisionEnabled` (`self.Sphere`) "QueryOnly")
      ;[1 1 1 0.5] 머리 흔들리면서 뒤로 물러나기
      (if (> _returnvalue_x_2 18089.0)
        (`self.K2_AddActorWorldOffset` (0.0 0.0 0.0))
        (if (`self.Delayed`)
          (set `self.HeadState` "NewEnumerator2"))
        (else
          (`self.K2_AddActorLocalOffset` (10.0 0.0 0.0)))))
    (:`NewEnumerator2`
      (set `self.Is Particle` false)
      (`PrimitiveComponent.SetCollisionEnabled` (`self.Sphere`) "NoCollision")
      ;[1 1 1 0.5] 날아가기
      (if (> _returnvalue_x 23262.0)
        (`self.K2_AddActorWorldOffset` (0.0 0.0 0.0))
        (`self.K2_SetActorRotation` (struct))
        (bind _outactors (`GameplayStatics.GetAllActorsOfClass` "/Game/NSE_New/Blueprints/BP_LeftHand_Cha.BP_LeftHand_Cha_C"))
        (set `/Game/NSE_New/Blueprints/BP_LeftHand_Cha.State_Attack3` "NewEnumerator2" (`|GetArrayItem` _outactors))
        (`KismetSystemLibrary.Delay` 1.0)
        (`|ExecutionSequence`
          (:`then_0`
            (bind _outactors_2 (`GameplayStatics.GetAllActorsOfClass` "/Game/NSE_New/Blueprints/BP_LeftHand_Cha.BP_LeftHand_Cha_C"))
            (set `/Game/NSE_New/Blueprints/BP_LeftHand_Cha.Attack_All` "NewEnumerator3" (`|GetArrayItem` _outactors_2)))
          (:`then_1`
            (bind _outactors_3 (`GameplayStatics.GetAllActorsOfClass` "/Game/NSE_New/Blueprints/BP_RightHand.BP_RightHand_C"))
            (set `/Game/NSE_New/Blueprints/BP_RightHand.Attack_All` "NewEnumerator3" (`|GetArrayItem` _outactors_3))))
        (else
          (`self.K2_AddActorWorldOffset` (100.0 0.0 0.0))
          (`self.K2_AddActorLocalRotation` (struct :`Pitch` -10.0)))))
    (:`NewEnumerator4`
      (`PrimitiveComponent.SetCollisionEnabled` (`self.Sphere`) "NoCollision")
      (`self.StartLoc`))))

(fn `StartLoc`
  (`self.K2_SetActorLocation` (+ (`self.K2_GetActorLocation`) (* (`KismetMathLibrary.Normal` (- (`KismetMathLibrary.MakeVector` 17524.0 -39.0 326.0) (`self.K2_GetActorLocation`))) 2000.0 (`GameplayStatics.GetWorldDeltaSeconds`))))
  (return))

(fn `UserConstructionScript`)