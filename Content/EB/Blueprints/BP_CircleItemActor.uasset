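; BP_CircleItemActor is a circle item that bobs its Circle1 component up and down with a sine wave on Tick while IsDestroy is true.
; Overlap by a BP_CircleDestroyActor1 spawns a BP_CircleDestroyActor at the item's location.
; Any overlap also lowers Circle1, hides Circledestroy and stops the bobbing.
; After a short Delay, the item raises Circle1, shows Circledestroy and resumes bobbing.
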(event `self.ReceiveActorBeginOverlap`
  (params (OtherActor :type "Actor Object Reference"))
  (`|ExecutionSequence`
    (:`then_0`
      (cast `/Game/EB/Blueprints/BP_CircleDestroyActor1` OtherActor)
      (`|SpawnActorFromClass` "/Game/EB/Blueprints/BP_CircleDestroyActor.BP_CircleDestroyActor_C" (`KismetMathLibrary.MakeTransform` (`self.K2_GetActorLocation`)) "Undefined" "MultiplyWithRoot" null null))
    (:`then_1`
      (`SceneComponent.K2_SetRelativeLocation` (`self.circle1`) (0.0 0.0 0.0) false false)
      (`SceneComponent.SetHiddenInGame` (`self.circledestroy`) true false)
      (set `self.isDestroy` false)
      (`KismetSystemLibrary.Delay` 3.5)
      (`SceneComponent.K2_SetRelativeLocation` (`self.circle1`) (0.0 0.0 44.0) false false)
      (`SceneComponent.SetHiddenInGame` (`self.circledestroy`) false false)
      (set `self.isDestroy` true))))

(event `self.ReceiveTick`
  (params (DeltaSeconds :type "Float (single-precision)"))
  ;[1 1 1] 윗부분 위아래로 자동 이동
  (if (`self.isDestroy`)
    (bind _output_get (set `self.C1Y` (+ (* DeltaSeconds 20.0) (`self.C1Y`))))
    (bind _output_get_2 (set `self.new location1` (`KismetMathLibrary.MakeVector` (.x (`SceneComponent.K2_GetComponentLocation` (`self.circle1`))) (.y (`SceneComponent.K2_GetComponentLocation` (`self.circle1`))) (+ (* (`KismetMathLibrary.Sin` _output_get) 0.7) (.z (`SceneComponent.K2_GetComponentLocation` (`self.circle1`)))))))
    (`SceneComponent.K2_SetWorldLocation` (`self.circle1`) _output_get_2 false false)))

(fn `UserConstructionScript`)