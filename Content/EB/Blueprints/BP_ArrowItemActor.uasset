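; BP_ArrowItemActor is an arrow item that plays a short animation when any actor overlaps it.
; Overlap sets IsAttack, so Tick pushes the Arrow along X, raises both cylinders and spins them faster in opposite directions.
; A Delay in Tick clears the flag after half a second, returning parts to rest positions with a slow idle spin.
; The accumulated offsets are never reset, and a BP_MarioHat_1 cast is unconnected.
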(event `self.ReceiveBeginPlay`)

(event `self.ReceiveActorBeginOverlap`
  (params (OtherActor :type "Actor Object Reference"))
  (set `self.isAttack` true))

(event `self.ReceiveTick`
  (params (DeltaSeconds :type "Float (single-precision)"))
  (if (`self.isAttack`)
    (`SceneComponent.K2_AddLocalRotation` (`self.Cylinder2`) (struct :`Yaw` 5.0) false false)
    (`SceneComponent.K2_AddLocalRotation` (`self.Cylinder3`) (struct :`Yaw` -5.0) false false)
    (bind _output_get (set `self.plusAX` (+ (`self.plusAX`) 0.5)))
    (`SceneComponent.K2_SetRelativeLocation` (`self.arrow`) (`KismetMathLibrary.MakeVector` _output_get) false false)
    (bind _output_get_2 (set `self.plusCY` (+ (`self.plusCY`) 0.5)))
    (`SceneComponent.K2_SetRelativeLocation` (`self.Cylinder3`) (`KismetMathLibrary.MakeVector` -35.0 -27.0 _output_get_2) false false)
    (bind _output_get_3 (set `self.plusCY2` (+ (`self.plusCY2`) 0.5)))
    (`SceneComponent.K2_SetRelativeLocation` (`self.Cylinder2`) (`KismetMathLibrary.MakeVector` -35.0 33.0 _output_get_3) false false)
    (`KismetSystemLibrary.Delay` 0.5)
    (set `self.isAttack` false)
    (else
      (`SceneComponent.K2_SetRelativeLocation` (`self.arrow`) (0.0 0.0 0.0) false false)
      (`SceneComponent.K2_SetRelativeLocation` (`self.Cylinder3`) (-35.0 -27.0 6.6) false false)
      (`SceneComponent.K2_SetRelativeLocation` (`self.Cylinder2`) (-35.0 33.0 6.6) false false)
      (`SceneComponent.K2_AddLocalRotation` (`self.Cylinder2`) (struct :`Yaw` 1.0) false false)
      (`SceneComponent.K2_AddLocalRotation` (`self.Cylinder3`) (struct :`Yaw` -1.0) false false))))

(fn `UserConstructionScript`)