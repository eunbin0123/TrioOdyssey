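; BP_CircleDestroyActor is a flat, expanding circle hazard that damages BP_ToBeMario on overlap, taking one HP and setting its damage flag.
; Tick advances a frame-rate-dependent timer that feeds an unclamped Lerp, steadily widening X and Y while Z stays thin.
; At the time limit it destroys itself with a whoosh sound, while another swoosh plays shortly after spawn.
; Logic for killing Gumbas and awarding coins is present but disconnected.
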(event `self.ReceiveBeginPlay`
  (`KismetSystemLibrary.Delay` 1.5)
  (`GameplayStatics.PlaySound2D` "/Game/EB/Sounds/swoosh-6428.swoosh-6428" 1.0 1.0 0.0 null null))

(event `self.ReceiveActorBeginOverlap`
  (params (OtherActor :type "Actor Object Reference"))
  (`|ExecutionSequence`
    (:`then_0`
      (bind _asbp_to_be_mario (cast `/Game/CJWCharactor/ThirdPerson/Blueprints/BP_ToBeMario` OtherActor))
      (set `/Game/CJWCharactor/ThirdPerson/Blueprints/BP_ToBeMario.IsGetDamage` true _asbp_to_be_mario)
      (bind _output_get (set `/Game/CJWCharactor/ThirdPerson/Blueprints/BP_ToBeMario.Hp` (- (`/Game/CJWCharactor/ThirdPerson/Blueprints/BP_ToBeMario.Hp` _asbp_to_be_mario) 1.0) _asbp_to_be_mario))
      (`KismetSystemLibrary.PrintString` (`KismetStringLibrary.Conv_DoubleToString` _output_get)))))

(event `self.ReceiveTick`
  (params (DeltaSeconds :type "Float (single-precision)"))
  (bind _returnvalue (`KismetMathLibrary.Lerp` 1.0 2.0 (`self.CurrentTime`)))
  (set `self.CurrentTime` (+ (`self.CurrentTime`) DeltaSeconds 0.1))
  (if (>= (`self.CurrentTime`) 25.0)
    (`self.K2_DestroyActor`)
    (`GameplayStatics.PlaySound2D` "/Game/EB/Sounds/fire-torch-whoosh-2-186586.fire-torch-whoosh-2-186586" 1.0 1.0 0.0 null null)
    (else
      (`self.SetActorScale3D` (`KismetMathLibrary.MakeVector` _returnvalue _returnvalue 0.01)))))

(fn `UserConstructionScript`)