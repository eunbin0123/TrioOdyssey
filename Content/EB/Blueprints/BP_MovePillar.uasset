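; BP_MovePillar is an actor that travels once along a spline path when play begins.
; It takes the spline from the BP_Move actor found in the level, then runs the Move timeline at a rate set by Speed.
; Each update maps the timeline alpha to spline distance, setting world location and local-space yaw while using the Box's relative scale.
; The finish event only runs a short delay with nothing after it.
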(event `self.ReceiveBeginPlay`
  (bind _returnvalue (`GameplayStatics.GetActorOfClass` "/Game/EB/Blueprints/BP_Move.BP_Move_C"))
  (set `self.SelectSpline` _returnvalue)
  (`self.MoveBox`))

(event `MoveBox`
  (`TimelineComponent.SetPlayRate` (`self.move`) (`self.Speed`))
  (bind (_direction _move) (`Timeline|move`)
    (:`Update`
      (bind _returnvalue (`KismetMathLibrary.Lerp` 0.0 (`SplineComponent.GetSplineLength` (`/Game/EB/Blueprints/BP_Move.Spline` (`self.SelectSpline`))) _move))
      (bind (_returnvalue_roll _returnvalue_pitch _returnvalue_yaw) (`KismetMathLibrary.BreakRotator` (`SplineComponent.GetRotationAtDistanceAlongSpline` (`/Game/EB/Blueprints/BP_Move.Spline` (`self.SelectSpline`)) _returnvalue "Local")))
      (`self.K2_SetActorTransform` (`KismetMathLibrary.MakeTransform` (`SplineComponent.GetLocationAtDistanceAlongSpline` (`/Game/EB/Blueprints/BP_Move.Spline` (`self.SelectSpline`)) _returnvalue "World") (`KismetMathLibrary.MakeRotator` 0.0 0.0 _returnvalue_yaw) (`SceneComponent.RelativeScale3D` (`self.Box`)))))
    (:`Finished`
      (`KismetSystemLibrary.Delay` 0.2))))

(fn `UserConstructionScript`)