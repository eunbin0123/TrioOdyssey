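; BP_SplineBox2 is an actor that travels along the spline of a BP_Spline2 actor found in the level on BeginPlay.
; The Move timeline, with play rate set by Speed, interpolates distance from zero to the spline's length.
; Each update places the actor at that world-space point and takes only yaw from the spline's local-space rotation.
; When the timeline finishes, a short delay runs with nothing after it.
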(event `self.ReceiveBeginPlay`
  (bind _returnvalue (`GameplayStatics.GetActorOfClass` "/Game/EB/Blueprints/BP_Spline2.BP_Spline2_C"))
  (set `self.SelectSpline` _returnvalue)
  (`self.MoveBox`))

(event `MoveBox`
  (`TimelineComponent.SetPlayRate` (`self.move`) (`self.Speed`))
  (bind (_direction _move) (`Timeline|move`)
    (:`Update`
      (bind _returnvalue (`KismetMathLibrary.Lerp` 0.0 (`SplineComponent.GetSplineLength` (`/Game/EB/Blueprints/BP_Spline2.Spline` (`self.SelectSpline`))) _move))
      (bind (_returnvalue_roll _returnvalue_pitch _returnvalue_yaw) (`KismetMathLibrary.BreakRotator` (`SplineComponent.GetRotationAtDistanceAlongSpline` (`/Game/EB/Blueprints/BP_Spline2.Spline` (`self.SelectSpline`)) _returnvalue "Local")))
      (`self.K2_SetActorTransform` (`KismetMathLibrary.MakeTransform` (`SplineComponent.GetLocationAtDistanceAlongSpline` (`/Game/EB/Blueprints/BP_Spline2.Spline` (`self.SelectSpline`)) _returnvalue "World") (`KismetMathLibrary.MakeRotator` 0.0 0.0 _returnvalue_yaw))))
    (:`Finished`
      (`KismetSystemLibrary.Delay` 0.2))))

(fn `UserConstructionScript`)