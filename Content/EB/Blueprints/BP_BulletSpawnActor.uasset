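; BP_BulletSpawnActor is a one-shot spawner that launches a BP_Roket when BP_ToBeMario comes within range.
; Until it has fired, Tick runs through a one-second Delay, then finds BP_ToBeMario by class and checks its distance against a fixed threshold.
; The rocket spawns at the Arrow component's location without its rotation, and the IsSpawn flag then blocks further spawns.
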(event `self.ReceiveBeginPlay`)

(event `self.ReceiveTick`
  (params (DeltaSeconds :type "Float (single-precision)"))
  (if (not (`self.isSpawn`))
    (`KismetSystemLibrary.Delay` 1.0)
    (bind _returnvalue (`GameplayStatics.GetActorOfClass` "/Game/CJWCharactor/ThirdPerson/Blueprints/BP_ToBeMario.BP_ToBeMario_C"))
    (if (<= (`self.GetDistanceTo` _returnvalue) 2300.0)
      (`|SpawnActorFromClass` "/Game/CJW/Blueprints/BP_Roket.BP_Roket_C" (`KismetMathLibrary.Conv_VectorToTransform` (`SceneComponent.K2_GetComponentLocation` (`self.Arrow`))) "Undefined" "MultiplyWithRoot" null null)
      (set `self.isSpawn` true))))

(fn `UserConstructionScript`)