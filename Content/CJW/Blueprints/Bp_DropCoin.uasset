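; Dropped coin actor that spins while drifting in a straight line with a timeline-driven vertical motion.
; BeginPlay starts the timeline, which adds its track value to the current Z each update, and caches the forward vector.
; Tick rotates the coin by a fixed, frame-rate-dependent step and moves it along the cached direction without sweep, scaled by delta time.
; No pickup or overlap logic is active.
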(event `self.ReceiveBeginPlay`
  (bind (_returnvalue_x _returnvalue_y _returnvalue_z) (`KismetMathLibrary.BreakVector` (`self.K2_GetActorLocation`)))
  (`|ExecutionSequence`
    (:`then_0`
      (bind (_direction _newtrack_0) (`Timeline|Timeline`)
        (:`Update`
          (`self.K2_SetActorLocation` (`KismetMathLibrary.MakeVector` _returnvalue_x _returnvalue_y (+ _returnvalue_z _newtrack_0))))))
    (:`then_1`
      (set `self.NewVar` (* (`self.GetActorForwardVector`) 1.0)))))

(event `self.ReceiveTick`
  (params (DeltaSeconds :type "Float (single-precision)"))
  (`self.K2_AddActorWorldRotation` (struct :`Yaw` 5.0))
  (`self.K2_SetActorLocation` (+ (`self.K2_GetActorLocation`) (* (`self.NewVar`) (`GameplayStatics.GetWorldDeltaSeconds`) 200.0))))

(fn `UserConstructionScript`)