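; Mario's thrown cap: a spinning projectile with a star trail that homes back to the player and acts on whatever it overlaps.
; Tick either moves it along a stored arrow direction or, after short delays, calls GoToMario to enable homing on the player's capsule.
; An overlap cast chain handles catching, redirection by arrow items, circle items, coin pickup, jump flowers, and capture of rockets, Gumbas and a left-hand boss.
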(event `GoToMario`
  (bind _projectilemovement (`self.ProjectileMovement`))
  ;[1 1 1] Go To Mario
  (set `ProjectileMovementComponent.HomingTargetComponent` (`Character.CapsuleComponent` (`GameplayStatics.GetPlayerCharacter` 0)) _projectilemovement)
  (set `ProjectileMovementComponent.bIsHomingProjectile` true _projectilemovement)
  (set `ProjectileMovementComponent.HomingAccelerationMagnitude` 8000.0 _projectilemovement))

(event `self.ReceiveTick`
  (params (DeltaSeconds :type "Float (single-precision)"))
  (`|ExecutionSequence`
    (:`then_0`
      (`self.K2_AddActorWorldRotation` (struct :`Yaw` 40.0) true))
    (:`then_1`
      (if (`self.isEnd`)
        ;[1 1 1] Arrow 따라서 모자 이동
        (`KismetSystemLibrary.Delay` 0.001)
        (`self.K2_SetActorLocation` (+ (`self.K2_GetActorLocation`) (* (`self.ArrowFirePosition`) (`self.Speed`) (`GameplayStatics.GetWorldDeltaSeconds`))))
        (set `self.isEnd` true)
        (else
          ;[1 1 1] 되돌아오는 모자
          (`KismetSystemLibrary.Delay` 0.0004)
          (`self.GoToMario`))))
    (:`then_2`
      ;[1 1 1] 모자 이펙트
      (`KismetSystemLibrary.Delay` 0.005)
      (`NiagaraFunctionLibrary.SpawnSystemAtLocation` "/Game/CJW/Particle/HatStarEffect.HatStarEffect" (`SceneComponent.K2_GetComponentLocation` (`self.Arrow1`))))
    (:`then_3`
      ;[1 1 1] 모자 던졌을 때 멈춤
      (if (`self.Stopduring`)
        (if (not (`self.isEnd`))
          (`self.GoToMario`))
        (else
          (`KismetSystemLibrary.Delay` 0.2)
          (`MovementComponent.StopMovementImmediately` (`self.CharacterMovement`))
          (`MovementComponent.StopMovementImmediately` (`self.ProjectileMovement`))
          (`KismetSystemLibrary.Delay` 0.3)
          (set `self.Stopduring` true))))))

(event `self.ReceiveActorBeginOverlap`
  (params (OtherActor :type "Actor Object Reference"))
  (`|ExecutionSequence`
    (:`then_0`
      ;[1 1 1] 플레이어 한테 맞으면 다시 모자 회수
      (bind _asbp_to_be_mario (cast `/Game/CJWCharactor/ThirdPerson/Blueprints/BP_ToBeMario` OtherActor)
        (:`then`
          (set `/Game/CJWCharactor/ThirdPerson/Blueprints/BP_ToBeMario.IsExistHat` false _asbp_to_be_mario)
          (`self.K2_DestroyActor`))
        (:`CastFailed`
          ;[1 1 1] 모자를 던졌을때 만약 로켓과 오버랩 되면, 빙의 가능 상태라면  우선 모자를 파괴하고 , 로켓의 플레이어 컨트롤러 모드를 킨다. 그게 아니라면 그 자리에서 되돌아온다
          (bind _asbp_roket (cast `/Game/CJW/Blueprints/BP_Roket` OtherActor))
          (if (`/Game/CJW/Blueprints/BP_Roket.IsEnablePossess` _asbp_roket)
            (`self.K2_DestroyActor`)
            (set `/Game/CJW/Blueprints/BP_Roket.IsPlayerControllerMode` true _asbp_roket)
            (bind _returnvalue (`GameplayStatics.GetActorOfClass` "/Game/CJWCharactor/ThirdPerson/Blueprints/BP_ToBeMario.BP_ToBeMario_C"))
            (bind _asbp_to_be_mario_2 (cast `/Game/CJWCharactor/ThirdPerson/Blueprints/BP_ToBeMario` _returnvalue))
            (`PrimitiveComponent.SetCollisionEnabled` (`Character.CapsuleComponent` _asbp_to_be_mario_2) "NoCollision")
            (`SceneComponent.SetVisibility` (`Character.Mesh` _asbp_to_be_mario_2) false false)
            (else
              (`PrimitiveComponent.SetCollisionEnabled` (`self.CapsuleComponent`) "NoCollision")
              (`MovementComponent.StopMovementImmediately` (`self.ProjectileMovement`))
              (`self.GoToMario`)
              (`KismetSystemLibrary.Delay` 0.3)
              (`PrimitiveComponent.SetCollisionEnabled` (`self.CapsuleComponent`) "QueryAndPhysics"))))))
    (:`then_1`
      ;[1 1 1] ArrowItem과 충돌시 방향 따라 이동* 바꿈
      (bind _asbp_arrow_item_actor (cast `/Game/EB/Blueprints/BP_ArrowItemActor` OtherActor))
      (set `ProjectileMovementComponent.bIsHomingProjectile` false (`self.ProjectileMovement`))
      (`MovementComponent.StopMovementImmediately` (`self.ProjectileMovement`))
      (bind _output_get (set `self.ArrowFirePosition` (`KismetMathLibrary.Conv_RotatorToVector` (`self.K2_GetActorRotation` _asbp_arrow_item_actor))))
      (bind _returnvalue_2 (`GameplayStatics.GetActorOfClass` "/Game/CJWCharactor/ThirdPerson/Blueprints/BP_ToBeMario.BP_ToBeMario_C"))
      (cast `/Game/CJWCharactor/ThirdPerson/Blueprints/BP_ToBeMario` _returnvalue_2)
      (`MovementComponent.StopMovementImmediately` (`self.ProjectileMovement`))
      (`self.K2_SetActorLocationAndRotation` (`self.K2_GetActorLocation` _asbp_arrow_item_actor) (`KismetMathLibrary.Conv_VectorToRotator` _output_get))
      (set `self.Stopduring` false)
      (set `self.isEnd` true)
      (`KismetSystemLibrary.Delay` 0.1)
      (set `self.Speed` 1500.0))
    (:`then_2`
      ;[1 1 1] CircleItem과 충돌시 CircleDestroy
      (bind _asbp_circle_item_actor (cast `/Game/EB/Blueprints/BP_CircleItemActor` OtherActor))
      (`|SpawnActorFromClass` "/Game/EB/Blueprints/BP_CircleDestroyActor.BP_CircleDestroyActor_C" (`KismetMathLibrary.MakeTransform` (`self.K2_GetActorLocation` _asbp_circle_item_actor)) "Undefined" "MultiplyWithRoot" null null)
      (bind _returnvalue_3 (`GameplayStatics.GetActorOfClass` "/Game/CJWCharactor/ThirdPerson/Blueprints/BP_ToBeMario.BP_ToBeMario_C"))
      (set `/Game/CJWCharactor/ThirdPerson/Blueprints/BP_ToBeMario.IsExistHat` false _returnvalue_3)
      (`self.K2_DestroyActor`)
      (set `self.isEnd` false)
      (set `self.Stopduring` true))
    (:`then_3`
      ;[1 1 1] Coin과 충돌 시 Coin 삭제
      (bind _asbp_coin_actor (cast `/Game/EB/Blueprints/BP_CoinActor` OtherActor))
      (`/Engine/EditorBlueprintResources/StandardMacros.IsValid` _asbp_coin_actor
        (:`Is Valid`
          (`GameplayStatics.PlaySound2D` "/Game/EB/Sounds/super-mario-odyssey-coin.super-mario-odyssey-coin" 1.0 1.0 0.0 null null)
          (`self.K2_DestroyActor` _asbp_coin_actor)
          (bind _returnvalue_4 (`GameplayStatics.GetActorOfClass` "/Game/CJWCharactor/ThirdPerson/Blueprints/BP_ToBeMario.BP_ToBeMario_C"))
          (bind _asbp_to_be_mario_3 (cast `/Game/CJWCharactor/ThirdPerson/Blueprints/BP_ToBeMario` _returnvalue_4))
          (set `/Game/CJWCharactor/ThirdPerson/Blueprints/BP_ToBeMario.Coin` (+ (`/Game/CJWCharactor/ThirdPerson/Blueprints/BP_ToBeMario.Coin` _asbp_to_be_mario_3) 1) _asbp_to_be_mario_3)
          (bind _ui (`/Game/CJWCharactor/ThirdPerson/Blueprints/BP_ToBeMario.Ui` _asbp_to_be_mario_3))
          (`UserWidget.PlayAnimation` _ui (`/Game/CJW/UI/MarioUi.GetCoin` _ui) 0.0 1 "Forward" 1.0 false))))
    (:`then_4`
      ;[1 1 1] Jump Flower과 충돌 시 점프 Active
      (bind _asbp_jump_flower (cast `/Game/EB/Blueprints/BP_JumpFlower` OtherActor))
      (set `/Game/EB/Blueprints/BP_JumpFlower.isJump` true _asbp_jump_flower)
      (`GameplayStatics.PlaySound2D` "/Game/EB/Sounds/squeakish-sound-102393.squeakish-sound-102393" 1.0 1.0 0.0 null null)
      (`|PlayMontage` (`/Game/EB/Blueprints/BP_JumpFlower.CapCatapult` _asbp_jump_flower) "/Game/EB/Resources/CapCatapult/Jump.Jump"
        (:`then`
          (`NiagaraFunctionLibrary.SpawnSystemAtLocation` "/Game/sA_PickupSet_1/Fx/NiagaraSystems/NS_CoinBurst.NS_CoinBurst"))))
    (:`then_5`
      (bind _asbp_gumba (cast `/Game/CJW/Blueprints/Gumba/BP_Gumba` OtherActor))
      (`/Game/CJW/Blueprints/Gumba/BP_Gumba.BePossesed` _asbp_gumba)
      (`self.K2_DestroyActor`)
      (bind _returnvalue_5 (`GameplayStatics.GetActorOfClass` "/Game/CJWCharactor/ThirdPerson/Blueprints/BP_ToBeMario.BP_ToBeMario_C"))
      (bind _asbp_to_be_mario_4 (cast `/Game/CJWCharactor/ThirdPerson/Blueprints/BP_ToBeMario` _returnvalue_5))
      (`PrimitiveComponent.SetCollisionEnabled` (`Character.CapsuleComponent` _asbp_to_be_mario_4) "NoCollision")
      (`SceneComponent.SetVisibility` (`Character.Mesh` _asbp_to_be_mario_4) false false))
    (:`then_6`
      (bind _asbp_left_hand_cha (cast `/Game/NSE_New/Blueprints/BP_LeftHand_Cha` OtherActor))
      (bind _canpossessed (`/Game/NSE_New/Blueprints/BP_LeftHand_Cha.CanPossessed` _asbp_left_hand_cha))
      (if _canpossessed
        (`Controller.Possess` (`GameplayStatics.GetPlayerController` 0) _asbp_left_hand_cha)
        (set `/Game/NSE_New/Blueprints/BP_LeftHand_Cha.Attack_All` "NewEnumerator2" _asbp_left_hand_cha)
        (bind _outactors (`GameplayStatics.GetAllActorsOfClass` "/Game/NSE_New/Blueprints/BP_RightHand.BP_RightHand_C"))
        (set `/Game/NSE_New/Blueprints/BP_RightHand.Attack_All` "NewEnumerator2" (`|GetArrayItem` _outactors))))))

(fn `UserConstructionScript`)