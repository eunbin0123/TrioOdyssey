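; Coin actor, named as a Gumba drop, that plays a short rising pop animation and then removes itself.
; On BeginPlay a timeline offsets its Z position each update while, after a brief delay, it destroys itself and plays the Super Mario Odyssey coin sound.
; Tick spins the coin around yaw and spawns a HatStarEffect system at the Arrow component every frame, with no overlap pickup logic.
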(event `self.ReceiveBeginPlay`
  (bind (_returnvalue_x _returnvalue_y _returnvalue_z) (`KismetMathLibrary.BreakVector` (`self.K2_GetActorLocation`)))
  (`|ExecutionSequence`
    (:`then_0`
      (bind (_direction _newtrack_0) (`Timeline|Timeline`)
        (:`Update`
          (`self.K2_SetActorLocation` (`KismetMathLibrary.MakeVector` _returnvalue_x _returnvalue_y (+ _returnvalue_z _newtrack_0))))))
    (:`then_1`
      (`KismetSystemLibrary.Delay` 0.8)
      (`self.K2_DestroyActor`)
      (`GameplayStatics.PlaySound2D` "/Game/EB/Sounds/super-mario-odyssey-coin.super-mario-odyssey-coin" 1.0 1.0 0.0 null null))))

(event `self.ReceiveTick`
  (params (DeltaSeconds :type "Float (single-precision)"))
  (`self.K2_AddActorWorldRotation` (struct :`Yaw` 25.0))
  (`NiagaraFunctionLibrary.SpawnSystemAtLocation` "/Game/CJW/Particle/HatStarEffect.HatStarEffect" (`SceneComponent.K2_GetComponentLocation` (`self.Arrow`))))

(fn `UserConstructionScript`)