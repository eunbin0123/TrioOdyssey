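; Right-hand boss actor that attacks the player in sync with its partner, BP_Left1.
; Tick runs a state machine for aiming and spawning BP_Ice, flipping and dropping downward, and chasing to perform repeated claps.
; It polls BP_Left1's state to trigger attacks and uses that hand's Y position to offset its chase target.
; Movement is stepped manually each frame with delta time, and distance checks advance the chase and clap phases.
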(event `self.ReceiveBeginPlay`)

(event `self.ReceiveActorBeginOverlap`
  (params (OtherActor :type "Actor Object Reference")))

(event `self.ReceiveTick`
  (params (DeltaSeconds :type "Float (single-precision)"))
  (bind (_returnvalue_x _returnvalue_y _returnvalue_z) (`KismetMathLibrary.BreakVector` (`self.K2_GetActorLocation`)))
  (bind (_returnvalue_x_2 _returnvalue_y_2) (`KismetMathLibrary.BreakVector` (`self.K2_GetActorLocation`)))
  (bind (_returnvalue_x_3 _returnvalue_y_3) (`KismetMathLibrary.BreakVector` (`self.K2_GetActorLocation`)))
  (bind (_returnvalue_x_4 _returnvalue_y_4) (`KismetMathLibrary.BreakVector` (`self.K2_GetActorLocation`)))
  (bind (_returnvalue_x_5 _returnvalue_y_5 _returnvalue_z_2) (`KismetMathLibrary.BreakVector` (`self.K2_GetActorLocation`)))
  (bind (_returnvalue_x_6 _returnvalue_y_6 _returnvalue_z_3) (`KismetMathLibrary.BreakVector` (`self.K2_GetActorLocation`)))
  (bind (_returnvalue_x_7 _returnvalue_y_7) (`KismetMathLibrary.BreakVector` (`self.K2_GetActorLocation`)))
  (bind (_returnvalue_x_8 _returnvalue_y_8 _returnvalue_z_4) (`KismetMathLibrary.BreakVector` (`self.K2_GetActorLocation`)))
  (bind _returnvalue_x_9 (`KismetMathLibrary.BreakVector` (`self.K2_GetActorLocation` (`GameplayStatics.GetPlayerPawn` 0))))
  (bind (_returnvalue_x_10 _returnvalue_y_9) (`KismetMathLibrary.BreakVector` (`self.K2_GetActorLocation` (`GameplayStatics.GetPlayerPawn` 0))))
  (bind (_returnvalue_x_11 _returnvalue_y_10) (`KismetMathLibrary.BreakVector` (`self.K2_GetActorLocation` (`GameplayStatics.GetPlayerPawn` 0))))
  (bind (_returnvalue_x_12 _returnvalue_y_11) (`KismetMathLibrary.BreakVector` (`self.K2_GetActorLocation` (`GameplayStatics.GetPlayerPawn` 0))))
  (bind _returnvalue_x_13 (`KismetMathLibrary.BreakVector` (`self.K2_GetActorLocation` (`GameplayStatics.GetPlayerPawn` 0))))
  (bind _returnvalue (`KismetMathLibrary.Vector_Distance` (`KismetMathLibrary.Conv_DoubleToVector` _returnvalue_y_3) (`KismetMathLibrary.Conv_DoubleToVector` _returnvalue_y_9)))
  (`|ExecutionSequence`
    (:`then_1`
      (switch `/Game/NSE/Modeling_Boss/Animations/EHandRightState` (`self.State`)
        (:`NewEnumerator1`
          ;[1 1 1] Spawn되면 Attack 호출
          (bind _returnvalue_2 (`GameplayStatics.GetActorOfClass` "/Game/NSE/Modeling_Boss/Blueprints/BP_Left1.BP_Left1_C"))
          (if (`|EnumEquality` (`/Game/NSE/Modeling_Boss/Blueprints/BP_Left1.State` _returnvalue_2) "NewEnumerator15")
            (`KismetSystemLibrary.Delay` 2.0)
            (set `self.State` "NewEnumerator5")))
        (:`NewEnumerator5`
          (`self.K2_SetActorRotation` (`KismetMathLibrary.RInterpTo` (`self.K2_GetActorRotation`) (`KismetMathLibrary.FindLookAtRotation` (`self.K2_GetActorLocation`) (`self.K2_GetActorLocation` (`GameplayStatics.GetPlayerPawn` 0))) DeltaSeconds 3.0))
          (`self.Make Ice`))
        (:`NewEnumerator12`
          (`self.Attack2`))
        (:`NewEnumerator13`
          (`self.Attack3`))
        (:`NewEnumerator14`
          (bind _outactors (`GameplayStatics.GetAllActorsOfClass` "/Game/NSE/Modeling_Boss/Blueprints/BP_Left1.BP_Left1_C"))
          (`self.K2_SetActorLocation` (`KismetMathLibrary.MakeVector` _returnvalue_x_2 _returnvalue_y_2 (`self.Return Value Z`)))
          ;[0.4853 0.6917 1] chase
          (`self.K2_SetActorRotation` (struct :`Pitch` 90.0 :`Roll` -90.0))
          (bind (_returnvalue_x_14 _returnvalue_y_12) (`KismetMathLibrary.BreakVector` (`self.K2_GetActorLocation` (`|GetArrayItem` _outactors))))
          (bind _returnvalue_3 (- _returnvalue_y_11 (/ (- _returnvalue_y_12 _returnvalue_y_7) 2.0)))
          (bind _returnvalue_4 (`KismetMathLibrary.MakeVector` _returnvalue_x_9 _returnvalue_3 _returnvalue_z_4))
          ;;[1 1 1] 플레이어와의 거리가 2m 이내이면 멈춘다.
          (if (< (`KismetMathLibrary.Vector_Distance` (`self.K2_GetActorLocation`) _returnvalue_4) 5.0)
            (`self.K2_SetActorLocation` (`KismetMathLibrary.MakeVector` _returnvalue_x_13 _returnvalue_3 _returnvalue_z_2))
            (set `self.State` "NewEnumerator15")
            (else
              ;;[1 1 1] 이동하다가
              (`self.K2_SetActorLocation` (+ (`self.K2_GetActorLocation`) (* (`KismetMathLibrary.Normal` (- _returnvalue_4 (`self.K2_GetActorLocation`))) 400.0 (`GameplayStatics.GetWorldDeltaSeconds`)))))))
        (:`NewEnumerator15`
          ;[1 1 1] 박수치기
          (`self.K2_SetActorLocation` (+ (`self.K2_GetActorLocation`) (* (`KismetMathLibrary.Normal` (- (`KismetMathLibrary.MakeVector` _returnvalue_x_6 (- _returnvalue_y_10 _returnvalue_y_4) _returnvalue_z_3) (`self.K2_GetActorLocation`))) 1200.0 (`GameplayStatics.GetWorldDeltaSeconds`))))
          (if (< _returnvalue 200.0)
            (set `self.State` "NewEnumerator16")))
        (:`NewEnumerator16`
          ;[1 1 1] Up
          (`self.K2_SetActorRelativeLocation` (+ (`self.K2_GetActorLocation`) (* (`GameplayStatics.GetWorldDeltaSeconds`) 600.0 (`KismetMathLibrary.MakeVector` 0.0 -70.0))))
          (if (> _returnvalue 600.0)
            (set `self.Num Clap` (- (`self.Num Clap`) 1.0))
            (if (<= (`self.Num Clap`) 0.0)
              (`self.K2_SetActorLocation` (`KismetMathLibrary.MakeVector` _returnvalue_x -800.0 _returnvalue_z))
              (else
                (set `self.State` "NewEnumerator15")
                (`KismetSystemLibrary.Delay` 3.0)))))))
    (:`then_2`
      (bind _outactors_2 (`GameplayStatics.GetAllActorsOfClass` "/Game/NSE/Modeling_Boss/Blueprints/BP_Left1.BP_Left1_C"))
      (if (`|EnumEquality` (`/Game/NSE/Modeling_Boss/Blueprints/BP_Left1.State` (`|GetArrayItem` _outactors_2)) "NewEnumerator16")
        (set `self.State` "NewEnumerator12")))
    (:`then_3`
      (bind _outactors_3 (`GameplayStatics.GetAllActorsOfClass` "/Game/NSE/Modeling_Boss/Blueprints/BP_Left1.BP_Left1_C"))
      (if (`|EnumEquality` (`/Game/NSE/Modeling_Boss/Blueprints/BP_Left1.State` (`|GetArrayItem` _outactors_3)) "NewEnumerator18")
        (set `self.State` "NewEnumerator14")))))

(event `Make Ice`
  (bind (_returnvalue_location _returnvalue_rotation) (`KismetMathLibrary.BreakTransform` (`SceneComponent.K2_GetComponentToWorld` (`self.Arrow1`))))
  ;[1 1 1] Ice 생성
  (`KismetSystemLibrary.Delay` 1.0)
  (`|SpawnActorFromClass` "/Game/NSE_New/Blueprints/BP_Ice.BP_Ice_C" (`KismetMathLibrary.MakeTransform` _returnvalue_location _returnvalue_rotation) "Undefined" "MultiplyWithRoot" null null))

(fn `Attack2`
  (`self.K2_SetActorLocationAndRotation` (`self.K2_GetActorLocation`) (struct :`Yaw` 180.0))
  (set `self.State` "NewEnumerator13"))

(fn `Attack3`
  (bind (_returnvalue_x _returnvalue_y) (`KismetMathLibrary.BreakVector` (`self.K2_GetActorLocation`)))
  (bind (_returnvalue_x_2 _returnvalue_y_2 _returnvalue_z) (`KismetMathLibrary.BreakVector` (`self.K2_GetActorLocation`)))
  (`self.K2_SetActorRelativeLocation` (+ (`self.K2_GetActorLocation`) (* (`GameplayStatics.GetWorldDeltaSeconds`) 5.0 (`KismetMathLibrary.MakeVector` 0.0 0.0 -1200.0))))
  (if (< _returnvalue_z 5.0)
    (`self.K2_SetActorRelativeLocation` (`KismetMathLibrary.MakeVector` _returnvalue_x _returnvalue_y))))

(fn `Attack4_clap`)

(fn `UserConstructionScript`)