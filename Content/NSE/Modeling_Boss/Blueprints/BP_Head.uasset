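; BP_Head is a head actor, apparently a boss part, that follows the state of BP_Lefthand.
; Every Tick it looks up the first BP_Lefthand and, while that hand is in one specific state, snaps itself to a hard-coded transform and disables capsule physics simulation.
; A Translate helper offers frame-rate-independent movement without sweep but is not called here, and TargetPoint is an empty stub.
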(event `self.ReceiveActorBeginOverlap`
  (params (OtherActor :type "Actor Object Reference")))

(event `self.ReceiveTick`
  (params (DeltaSeconds :type "Float (single-precision)"))
  (bind _outactors (`GameplayStatics.GetAllActorsOfClass` "/Game/NSE/Modeling_Boss/Blueprints/BP_Lefthand.BP_Lefthand_C"))
  (if (`|EnumEquality` (`/Game/NSE/Modeling_Boss/Blueprints/BP_Lefthand.State` (`|GetArrayItem` _outactors)) "NewEnumerator16")
    (`|ExecutionSequence`
      (:`then_0`
        (`self.K2_SetActorLocationAndRotation` (7579.0 27.0 902.0) (struct :`Yaw` 180.0)))
      (:`then_1`
        (`PrimitiveComponent.SetSimulatePhysics` (`self.CapsuleComponent`) false)))))

(event `self.ReceiveAnyDamage`
  (params (Damage :type "Float (single-precision)") (DamageType :type "DamageType Object Reference") (InstigatedBy :type "Controller Object Reference") (DamageCauser :type "Actor Object Reference")))

(fn `Target Point`)

(fn `Translate`
  (params (Direction :type "Vector Structure") (Speed :type "Float (double-precision)"))
  (`self.K2_SetActorLocation` (+ (`self.K2_GetActorLocation`) (* Direction Speed (`GameplayStatics.GetWorldDeltaSeconds`)))))

(fn `UserConstructionScript`)