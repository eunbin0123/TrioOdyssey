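; BP_Test is a test actor in the boss modeling folder that slides along world Y each tick, driven by the first player pawn's position.
; It moves at a fixed speed without sweep, keeping X and Z constant.
; The target Y is the player's Y minus its own, so it settles around half the player's Y rather than matching it.
; A variant with the subtraction reversed is left unconnected.
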(event `self.ReceiveTick`
  (params (DeltaSeconds :type "Float (single-precision)"))
  (bind (_returnvalue_x _returnvalue_y) (`KismetMathLibrary.BreakVector` (`self.K2_GetActorLocation`)))
  (bind (_returnvalue_x_2 _returnvalue_y_2 _returnvalue_z) (`KismetMathLibrary.BreakVector` (`self.K2_GetActorLocation`)))
  (bind (_returnvalue_x_3 _returnvalue_y_3) (`KismetMathLibrary.BreakVector` (`self.K2_GetActorLocation` (`GameplayStatics.GetPlayerPawn` 0))))
  (`self.K2_SetActorLocation` (+ (`self.K2_GetActorLocation`) (* (`KismetMathLibrary.Normal` (- (`KismetMathLibrary.MakeVector` _returnvalue_x_2 (- _returnvalue_y_3 _returnvalue_y) _returnvalue_z) (`self.K2_GetActorLocation`))) 1200.0 (`GameplayStatics.GetWorldDeltaSeconds`)))))

(fn `UserConstructionScript`)